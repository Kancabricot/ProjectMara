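; Trigger-box actor that plays a one-time cinematic when the first-person character enters while it is active, then starts a monster's spline chase.
; It disables input, blends the view to a camera, plays the level sequence and waits out its duration.
; Afterwards it applies the camera rotation captured just before the end, moves the original view target to a hard-coded location, blends back and restores player input and position.
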(event OnComponentBeginOverlap(Box)
  (params (OverlappedComponent :type Primitive%20Component%20Object%20Reference) (OtherActor :type Actor%20Object%20Reference) (OtherComp :type Primitive%20Component%20Object%20Reference) (OtherBodyIndex :type Integer) (bFromSweep :type Boolean) (SweepResult :type Hit%20Result%20Structure%20%28by%20ref%29))
  (if (Variables|Default|GetIsActive)
    (bind _asbp_first_person_character (Utilities|Casting|CastToBP_FirstPersonCharacter OtherActor))
    (Variables|Default|SetPlayerRef _asbp_first_person_character)
    (if (not (Variables|Default|GetHasPlayed))
      (CallFunction|EnterCine)
      (Variables|Default|SetHasPlayed true))))

(event Custom|EnterCine
  (bind _returnvalue (Game|GetPlayerController 0))
  (bind _returnvalue_2 (Game|GetPlayerController 0))
  (bind _sequencertoplay (Variables|Default|GetSequencerToPlay))
  (bind _playerref (Variables|Default|GetPlayerRef))
  (bind _sequenceplayer (Variables|/Script/LevelSequence.LevelSequenceActor|GetSequencePlayer _sequencertoplay))
  (bind _returnvalue_3 (Media|MediaPlayer|GetDuration _sequenceplayer))
  (bind _returnvalue_4 (Class|TimeManagementBlueprintLibrary|ToSeconds(QualifiedFrameTime) _returnvalue_3))
  (Variables|Default|SetPlayerPos (Transformation|GetActorLocation (Variables|Default|GetPlayerRef)))
  (Input|DisableInput (Variables|Default|GetPlayerRef) _returnvalue_2)
  (Variables|Default|SetcamReturd (Pawn|GetViewTarget _returnvalue_2))
  (Game|Player|SetViewTargetwithBlend _returnvalue_2 (Variables|Default|GetCamToBlend) (Variables|Default|GetBlendTime) "VTBlend_Linear" 0.0 false)
  (Sequencer|Player|Play _sequenceplayer :!class /Script/MovieScene.MovieSceneSequencePlayer)
  (Utilities|FlowControl|Sequence
    (:then_0
      (Utilities|FlowControl|Delay _returnvalue_4)
      (Pawn|SetControlRotation (Pawn|GetController (Variables|/Script/Engine.Actor|GetInstigator _playerref)) (Variables|Default|GetrotTP))
      (Transformation|SetActorLocation (Variables|Default|GetcamReturd) "2020.000000,-2630.000000,10778.000000" false false)
      (Game|Player|SetViewTargetwithBlend _returnvalue (Variables|Default|GetcamReturd) (Variables|Default|GetBlendTime) "VTBlend_Linear" 0.0 false)
      (Input|EnableInput (Variables|Default|GetPlayerRef) _returnvalue)
      (Transformation|SetActorLocation _playerref (Variables|Default|GetPlayerPos) false false)
      (Default|ChaseAroundSpline (Variables|Default|GetMonster) (Variables|Default|GetSpline)))
    (:then_1
      (Utilities|FlowControl|Delay (- _returnvalue_4 0.1))
      (Variables|Default|SetrotTP (Transformation|GetActorRotation (Variables|Default|GetCamToBlend))))))

(event EventBeginPlay)

(event Collision|EventActorBeginOverlap
  (params (OtherActor :type Actor%20Object%20Reference)))

(event EventTick
  (params (DeltaSeconds :type Float%20%28single-precision%29)))

(fn ConstructionScript)