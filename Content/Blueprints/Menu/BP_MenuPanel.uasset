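; BP_MenuPanel is a menu panel actor hosting a WG_Menu widget and linked to other panels for navigation.
; The widget's transition event supplies an index into LinkedMenus, and the player's view blends to that panel with eased timing.
; Collision is off from BeginPlay and enabled only on the destination after the blend.
; The destination widget then gets a focus message, while all other cached panels get unfocus messages.
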(event Custom|Transition%20To
  (params (New%20Menu :type BP%20Menu%20Panel%20Object%20Reference))
  ;[1 1 1] Transition
  (Collision|SetActorEnableCollision false)
  (Game|Player|SetViewTargetwithBlend (Game|GetPlayerController 0) New%20Menu (Variables|Default|GetBlend%20Time) "VTBlend_EaseInOut" 2.0 false)
  (Utilities|FlowControl|Delay (Variables|Default|GetBlend%20Time))
  (Collision|SetActorEnableCollision New%20Menu true)
  (Class|BPIMenu|Focus(Message) (UserInterface|GetWidget (Variables|BP_MenuPanel_C|GetWidget New%20Menu)))
  (for _array_element (Variables|Default|GetArrayPanel)
    (if (== _array_element New%20Menu)
      (Development|PrintString "Same Widget")
      (else
        (Class|BPIMenu|Unfocus(Message) (UserInterface|GetWidget (Variables|BP_MenuPanel_C|GetWidget _array_element)))))))

(event Custom|OnTransitionsBetweenMenus
  (params (Index%20Menu :type Integer))
  ;[1 1 1] Gestion des collisions
  (if (Utilities|Array|IsValidIndex (Variables|Default|GetLinkedMenus) Index%20Menu)
    (CallFunction|Transitionto (Utilities|Array|Get(acopy) (Variables|Default|GetLinkedMenus) Index%20Menu))))

(event EventBeginPlay
  ;[1 1 1] Gestion des collisions
  (bind _aswg_menu (Utilities|Casting|CastToWG_Menu (UserInterface|GetUserWidgetObject (Variables|Default|GetWidget))))
  (EventDispatchers|BindEventtoTransitiontoLinkedMenu _aswg_menu (delegate Custom|OnTransitionsBetweenMenus))
  (Collision|SetActorEnableCollision false)
  (bind _outactors (Actor|GetAllActorsOfClass "BP_MenuPanel_C"))
  (Variables|Default|SetArrayPanel _outactors))

(fn ConstructionScript)