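; BP_Show_Text is a trigger box that shows tutorial text on the cursor widget when the first-person character enters it.
; BeginPlay caches the first WG_PlayerCursor, and each overlap writes the current TextsToShow entry into TextTestTuto.
; Leaving advances IndexText but sets the text Visible, despite the comment saying it hides.
; The overflow check compares and indexes with the array length, so it misses the last valid entry.
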(event OnComponentBeginOverlap(Box)
  (params (OverlappedComponent :type Primitive%20Component%20Object%20Reference) (OtherActor :type Actor%20Object%20Reference) (OtherComp :type Primitive%20Component%20Object%20Reference) (OtherBodyIndex :type Integer) (bFromSweep :type Boolean) (SweepResult :type Hit%20Result%20Structure%20%28by%20ref%29))
  (bind _texts_to_show (Variables|Default|GetTexts%20to%20Show))
  (bind _texts_to_show_2 (Variables|Default|GetTexts%20to%20Show))
  ;[1 1 1] Set text to show and his Visibilty to Visible
  (Utilities|Casting|CastToBP_FirstPersonCharacter OtherActor)
  (if (> (Variables|Default|GetIndex%20text) (Utilities|Array|Length _texts_to_show_2))
    (Variables|/Script/UMG.TextBlock|SetText (Variables|/Game/Widget/WG_PlayerCursor.WG_PlayerCursor_C|GetText_Test_Tuto (Variables|Default|GetWG%20Ref)) (Utilities|Array|Get(acopy) _texts_to_show (Utilities|Array|Length _texts_to_show)))
    (else
      (Variables|/Script/UMG.TextBlock|SetText (Variables|/Game/Widget/WG_PlayerCursor.WG_PlayerCursor_C|GetText_Test_Tuto (Variables|Default|GetWG%20Ref)) (Utilities|Array|Get(acopy) _texts_to_show_2 (Variables|Default|GetIndex%20text)))
      (Widget|SetVisibility (Variables|/Game/Widget/WG_PlayerCursor.WG_PlayerCursor_C|GetText_Test_Tuto (Variables|Default|GetWG%20Ref)) "Visible"))))

(event OnComponentEndOverlap(Box)
  (params (OverlappedComponent :type Primitive%20Component%20Object%20Reference) (OtherActor :type Actor%20Object%20Reference) (OtherComp :type Primitive%20Component%20Object%20Reference) (OtherBodyIndex :type Integer))
  ;[1 1 1] Hide text To Show
  (Utilities|Casting|CastToBP_FirstPersonCharacter OtherActor)
  (Widget|SetVisibility (Variables|/Game/Widget/WG_PlayerCursor.WG_PlayerCursor_C|GetText_Test_Tuto (Variables|Default|GetWG%20Ref)) "Visible")
  (Variables|Default|SetIndex%20text (+ (Variables|Default|GetIndex%20text) 1)))

(event EventBeginPlay
  ;[1 1 1] get Widget ref
  (bind _foundwidgets (Widget|GetAllWidgetsOfClass "/Game/Widget/WG_PlayerCursor.WG_PlayerCursor_C" true))
  (Variables|Default|SetWG%20Ref (Utilities|Array|Get(acopy) _foundwidgets)))

(fn ConstructionScript)