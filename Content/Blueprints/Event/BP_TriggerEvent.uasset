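; BP_TriggerEvent is a box trigger that fires a scripted world event selected by WhatEvent.
; When BP_FirstPersonCharacter overlaps, it either zeroes one set of lights and brightens another after a delay, or enables physics on an object to make it fall.
; A parallel Sequence branch opens a linked door after a short delay if OpenDoor is set, without checking the overlapping actor.
; Nothing limits it to one firing.
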(event OnComponentBeginOverlap(Box)
  (params (OverlappedComponent :type Primitive%20Component%20Object%20Reference) (OtherActor :type Actor%20Object%20Reference) (OtherComp :type Primitive%20Component%20Object%20Reference) (OtherBodyIndex :type Integer) (bFromSweep :type Boolean) (SweepResult :type Hit%20Result%20Structure%20%28by%20ref%29))
  ;[1 1 1] Light
  (Utilities|FlowControl|Sequence
    (:then_0
      (Utilities|Casting|CastToBP_FirstPersonCharacter OtherActor)
      (switch int (Variables|Default|GetWhatEvent)
        (:1
          (for _array_element (Variables|Components|GetLightToTurnOff_1)
            (Rendering|Components|Light|SetIntensity (Variables|/Script/Engine.Light|GetLightComponent _array_element) 0.0))
          (Utilities|FlowControl|Delay 1.0)
          (for _array_element_2 (Variables|Components|GetLightToTurnOn)
            (Rendering|Components|Light|SetIntensity (Variables|/Script/Engine.Light|GetLightComponent _array_element_2) 17.0)))
        (:2
          (Physics|SetSimulatePhysics (Variables|/Script/Engine.StaticMeshActor|GetStaticMeshComponent (Variables|Default|GetObjectToFall)) true))))
    (:then_1
      (if (Variables|Default|GetOpenDoor)
        (Utilities|FlowControl|Delay 0.3)
        (Default|OpenScriptedDoor (Variables|Default|GetDoorToOpen%20))))))

(fn ConstructionScript)

(fn EventLight)