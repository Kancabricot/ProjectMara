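; BP_DoorKnock is a sound event that plays a door-banging sound when the first-person player stands inside its trigger box.
; BeginPlay caches the player character, and Tick polls the box for overlap with it.
; A 2.5-second Delay on Tick spaces the knocks, which repeat while the overlap lasts.
; Each knock plays at the Audio component's location and prints a debug string.
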(event EventBeginPlay
  ;[1 1 1] Frappage de porte
  (bind _returnvalue (Actor|GetActorOfClass "/Game/Blueprints/BP_FirstPersonCharacter.BP_FirstPersonCharacter_C"))
  (Variables|Default|SetPlayer _returnvalue))

(event EventTick
  (params (DeltaSeconds :type Float%20%28single-precision%29))
  ;[1 1 1] Frappage de porte
  (if (Collision|IsOverlappingActor (Variables|Default|GetBox) (Variables|Default|GetPlayer) :!class /Script/Engine.PrimitiveComponent)
    (Utilities|FlowControl|Delay 2.5)
    (Audio|PlaySoundatLocation "/Game/Assets/SFX/Ambiance/Door_bang_01_Cue.Door_bang_01_Cue" (Transformation|GetWorldLocation (Variables|Default|GetAudio)) "0, 0, 0" 1.0 1.0 0.0 0 0 0 0)
    (Development|PrintString "knock knock")))

(fn ConstructionScript)