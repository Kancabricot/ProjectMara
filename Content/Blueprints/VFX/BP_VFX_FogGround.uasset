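; BP_VFX_FogGround is a placeable VFX actor that wraps a Niagara system, named for ground fog.
; Its Construction Script pushes the Spawn Rate, Lifetime, Box Size and Color variables into the matching Niagara user parameters, so each instance is configured at construction.
; The Event Graph holds only disabled stub events, so the Blueprint adds no runtime logic.
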(event EventBeginPlay)

(event Collision|EventActorBeginOverlap
  (params (OtherActor :type Actor%20Object%20Reference)))

(event EventTick
  (params (DeltaSeconds :type Float%20%28single-precision%29)))

(fn ConstructionScript
  (Effects|Components|ParticleSystem|SetFloatParameter (Variables|Default|GetNiagara) "user.Spawn Rate" (Variables|EmiterParameter|GetSpawn%20Rate))
  (Effects|Components|ParticleSystem|SetFloatParameter (Variables|Default|GetNiagara) "user.Lifetime" (Variables|EmiterParameter|GetLifetime))
  (Effects|Components|ParticleSystem|SetVectorParameter (Variables|Default|GetNiagara) "user.Box Size" (Variables|EmiterParameter|GetBox%20Size))
  (Effects|Components|ParticleSystem|SetColorParameter (Variables|Default|GetNiagara) "user.Color" (Variables|EmiterParameter|GetColor)))