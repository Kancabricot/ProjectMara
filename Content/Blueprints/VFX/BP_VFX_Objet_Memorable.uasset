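; Niagara effect Blueprint for a memorable object ("Objet Memorable"), exposing the look of its particle effect as Blueprint variables.
; The Construction Script copies those variables into the Niagara component's user parameters, covering color, spawn rate, radius, gravity, and lifetime and size ranges.
; The file contains no runtime logic, only this construction-time parameter setup.
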(fn ConstructionScript
  (Effects|Components|ParticleSystem|SetColorParameter (Variables|Default|GetNiagara) "user.Color" (Variables|EmiterParameter|GetColor))
  (Effects|Components|ParticleSystem|SetFloatParameter (Variables|Default|GetNiagara) "user.Spawn Rate" (Variables|EmiterParameter|GetSpawn%20Rate))
  (Effects|Components|ParticleSystem|SetFloatParameter (Variables|Default|GetNiagara) "user.Radius" (Variables|EmiterParameter|GetRadius))
  (Effects|Components|ParticleSystem|SetVectorParameter (Variables|Default|GetNiagara) "user.Gravity" (Variables|EmiterParameter|GetGravity))
  (Effects|Components|ParticleSystem|SetFloatParameter (Variables|Default|GetNiagara) "user.Lifetime Min" (Variables|EmiterParameter|GetLifetime%20Min))
  (Effects|Components|ParticleSystem|SetFloatParameter (Variables|Default|GetNiagara) "user.Lifetime Max" (Variables|EmiterParameter|GetLifetime%20Max))
  (Effects|Components|ParticleSystem|SetFloatParameter (Variables|Default|GetNiagara) "user.Size Max" (Variables|EmiterParameter|GetSize%20MAx))
  (Effects|Components|ParticleSystem|SetFloatParameter (Variables|Default|GetNiagara) "user.Size Min" (Variables|EmiterParameter|GetSize%20Min)))