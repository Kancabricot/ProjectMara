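; BP_Sound is a trigger-based sound actor that plays a random sound, picked from an array at BeginPlay, when the first-person character enters its trigger.
; Each overlap decrements a use counter, and non-looping actors destroy themselves once it runs out, straight after starting playback.
; Looping actors replay when the audio finishes if the player still overlaps the trigger.
; A separate PlaySound event starts playback manually, with optional fade-in.
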(event OnComponentBeginOverlap(Trigger)
  (params (OverlappedComponent :type Primitive%20Component%20Object%20Reference) (OtherActor :type Actor%20Object%20Reference) (OtherComp :type Primitive%20Component%20Object%20Reference) (OtherBodyIndex :type Integer) (bFromSweep :type Boolean) (SweepResult :type Hit%20Result%20Structure%20%28by%20ref%29))
  (bind _asbp_first_person_character (Utilities|Casting|CastToBP_FirstPersonCharacter OtherActor))
  (Variables|Ref|SetPlayerRef _asbp_first_person_character)
  (Audio|Components|Audio|Play (Variables|Default|GetAudio) 0.0)
  (bind _output_get (Variables|Sound|SetNbTimeToUse (- (Variables|Sound|GetNbTimeToUse) 1)))
  (if (<= _output_get 0)
    (if (not (Variables|Sound|Getb_IsLoop))
      (Actor|DestroyActor))))

(event OnAudioFinished(Audio)
  (if (Variables|Sound|Getb_IsLoop)
    (if (Collision|IsOverlappingActor (Variables|Default|GetTrigger) (Variables|Ref|GetPlayerRef) :!class /Script/Engine.PrimitiveComponent)
      (Audio|Components|Audio|Play (Variables|Default|GetAudio) 0.0))))

(event Custom|PlaySound
  (Audio|Components|Audio|Play (Variables|Default|GetAudio) 0.0)
  (if (Variables|Sound|Getb_IsFade)
    (Audio|Components|Audio|FadeIn (Variables|Default|GetAudio) (Variables|Sound|GetFade%20in%20Duration) 1.0 0.0 "Linear" :!class /Script/Engine.AudioComponent)))

(event EventBeginPlay
  (Audio|Components|Audio|SetSound (Variables|Default|GetAudio) (.OutItem (Utilities|Array|Random (Variables|Sound|GetSound)))))

(fn ConstructionScript)