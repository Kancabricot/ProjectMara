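; Non-Euclidean window portal that shows the view from a linked target camera and teleports actors through it.
; Construction picks the render-target material by name and adds a spline to the target.
; While the player is inside the render trigger, Tick mirrors the player camera's relative transform onto the target camera.
; Overlapping actors teleport to that camera when a short view trace hits TargetView, and control rotation is matched.
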(event OnComponentBeginOverlap(TPtrigger)
  (params (OverlappedComponent :type Primitive%20Component%20Object%20Reference) (OtherActor :type Actor%20Object%20Reference) (OtherComp :type Primitive%20Component%20Object%20Reference) (OtherBodyIndex :type Integer) (bFromSweep :type Boolean) (SweepResult :type Hit%20Result%20Structure%20%28by%20ref%29))
  (Variables|Default|Setb_CheckTP true)
  (Variables|Default|SetActorToTPRef OtherActor))

(event OnComponentEndOverlap(TPtrigger)
  (params (OverlappedComponent :type Primitive%20Component%20Object%20Reference) (OtherActor :type Actor%20Object%20Reference) (OtherComp :type Primitive%20Component%20Object%20Reference) (OtherBodyIndex :type Integer))
  (Variables|Default|Setb_CheckTP false)
  (Variables|Default|SetActorToTPRef 0))

(event OnComponentBeginOverlap(TriggerForRender)
  (params (OverlappedComponent :type Primitive%20Component%20Object%20Reference) (OtherActor :type Actor%20Object%20Reference) (OtherComp :type Primitive%20Component%20Object%20Reference) (OtherBodyIndex :type Integer) (bFromSweep :type Boolean) (SweepResult :type Hit%20Result%20Structure%20%28by%20ref%29))
  ;[1 1 1] Suivant si le joueur est ou n'est pas dans la zone change le matérial du portail
  (Utilities|Casting|CastToBP_FirstPersonCharacter OtherActor)
  (Variables|Default|Setb_MustRender true)
  (if (not (Variables|Default|Getb_DontRenderedPortal))
    (Rendering|Material|SetMaterial (Variables|Default|GetPortal) 0 (Variables|Default|GetMaterialOfTargetCam))))

(event OnComponentEndOverlap(TriggerForRender)
  (params (OverlappedComponent :type Primitive%20Component%20Object%20Reference) (OtherActor :type Actor%20Object%20Reference) (OtherComp :type Primitive%20Component%20Object%20Reference) (OtherBodyIndex :type Integer))
  ;[1 1 1] Suivant si le joueur est ou n'est pas dans la zone change le matérial du portail
  (Utilities|Casting|CastToBP_FirstPersonCharacter OtherActor)
  (Variables|Default|Setb_MustRender false)
  (if (not (Variables|Default|Getb_DontRenderedPortal))
    (Rendering|Material|SetMaterial (Variables|Default|GetPortal) 0 "/Game/ModularProps/Material_002.Material_002")))

(event EventBeginPlay
  ;[1 1 1] Suivant si le joueur est ou n'est pas dans la zone change le matérial du portail
  (if (not (Variables|Default|Getb_DontRenderedPortal))
    (Rendering|Material|SetMaterial (Variables|Default|GetPortal) 0 "/Game/ModularProps/Material_002.Material_002")))

(event EventTick
  (params (DeltaSeconds :type Float%20%28single-precision%29))
  (bind _returnvalue (Game|GetPlayerCameraManager 0))
  (bind _transformcomponent (Variables|/Script/Engine.PlayerCameraManager|GetTransformComponent _returnvalue))
  (bind _returnvalue_2 (Transformation|GetWorldLocation _transformcomponent))
  (Utilities|FlowControl|Sequence
    (:then_0
      (if (Variables|Default|Getb_MustRender)
        (CallFunction|RenderCambyPlayer)))
    (:then_1
      (if (Variables|Default|Getb_CheckTP)
        (bind _outhit (Collision|BoxTraceByChannel _returnvalue_2 (+ _returnvalue_2 (* (Math|Vector|GetForwardVector _transformcomponent) 80)) "1.000000,1.000000,1.000000" "0, 0, 0" "TraceTypeQuery1" false 0 "None" false))
        (if (== (.HitComponent (Collision|BreakHitResult _outhit)) (Variables|Default|GetTargetView))
          (if (not (Variables|Default|Getb_CanNotTP))
            (CallFunction|TPActor (Variables|Default|GetActorToTPRef))))))))

(fn ConstructionScript
  (if (not (Variables|Default|Getb_DontRenderedPortal))
    ;[1 1 1] Si il y a une caméra target alors rajoute un trait entre eux et change son matérial suivant la texture de la cam
    (bind _targetcamref (Variables|Default|GetTargetCamRef)
      (:then
        (bind _returnvalue (AddComponent|AddSplineComponent false))
        (Spline|SetLocationatSplinePoint _returnvalue 1 (Transformation|GetWorldLocation (Variables|/Game/Blueprints/Non-Euclidian/BP_CamRenderer.BP_CamRenderer_C|GetDefaultSceneRoot _targetcamref)) "World" true)
        (CallFunction|SetPortalMaterial))
      (:else))
    (else
      ;[1 1 1] Détruit le rendu du matérial si on n'en as pas besoin
      (bind _portal (Variables|Default|GetPortal)
        (:then
          (Components|DestroyComponent _portal))
        (:else))))
  ;[1 1 1] Change entre visible et invisible suivant les besoins
  (if (not (Variables|Default|Getb_IsInvisible))
    (Rendering|SetVisibility (Variables|Default|GetDefaultSceneRoot) true true)
    (else
      (Rendering|SetVisibility (Variables|Default|GetDefaultSceneRoot) false true))))

(fn SetPortalMaterial
  (bind _array_element (Utilities|Array|ForEachLoopwithBreak (Variables|Default|GetMaterialCamTargetArray) :!label _label)
    (:LoopBody
      (if (Utilities|Enum|Equal(Enum) (Utilities|GetObjectName _array_element) (Variables|/Game/Blueprints/Non-Euclidian/BP_CamRenderer.BP_CamRenderer_C|GetNameofTextureTargetRender (Variables|Default|GetTargetCamRef)))
        (Variables|Default|SetMaterialOfTargetCam _array_element)
        (Rendering|Material|SetMaterial (Variables|Default|GetPortal) 0 _array_element)
        (goto _label Break)))))

(fn RenderCambyPlayer
  (bind _returnvalue (Game|GetPlayerCameraManager 0))
  (bind _camtarget (Variables|Default|GetCamTarget))
  (bind _transformcomponent (Variables|/Script/Engine.PlayerCameraManager|GetTransformComponent _returnvalue))
  ;[1 1 1] Met la target de la camera au niveau de la caméra du player
  (Transformation|SetWorldLocationAndRotation (Variables|Default|GetCamTarget) (Transformation|GetWorldLocation _transformcomponent) (Transformation|GetWorldRotation _transformcomponent) false false)
  ;[1 1 1] Change la position de la caméra qui nous donne la texture au niveau de la position relative de la cam target
  (Transformation|SetRelativeLocationAndRotation (Variables|/Game/Blueprints/Non-Euclidian/BP_CamRenderer.BP_CamRenderer_C|GetCamRenderer (Variables|Default|GetTargetCamRef)) (Variables|/Script/Engine.SceneComponent|GetRelativeLocation _camtarget) (Variables|/Script/Engine.SceneComponent|GetRelativeRotation _camtarget) false false))

(fn TPActor
  (params (TargetTP :type Actor%20Object%20Reference))
  (bind _targetcamref (Variables|Default|GetTargetCamRef))
  (bind _camrenderer (Variables|/Game/Blueprints/Non-Euclidian/BP_CamRenderer.BP_CamRenderer_C|GetCamRenderer _targetcamref))
  (bind _returnvalue (Transformation|GetWorldLocation _camrenderer))
  ;[1 1 1] Téléporte l'acteur au niveau de Camrenderer
  (Transformation|Teleport TargetTP (Math|Vector|MakeVector (+ (Variables|Default|GetOffsetTP) (.x _returnvalue)) (.y _returnvalue) (+ (.z _returnvalue) -151.327179)) "0, 0, 0")
  (Pawn|SetControlRotation (Game|GetPlayerController 0) (Transformation|GetWorldRotation _camrenderer))
  (return))