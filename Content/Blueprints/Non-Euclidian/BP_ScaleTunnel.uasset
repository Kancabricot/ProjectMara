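; Non-Euclidean tunnel that resizes the first-person player while they are inside its trigger box.
; BeginPlay caches the player and uses a line trace from Start to End to measure the maximum distance.
; During overlap, the Update timeline repeats a box trace along that axis, normalizes the hit distance and lerps player scale uniformly from 1 toward TailleMin.
; Leaving the box stops the updates without resetting the scale.
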(event OnComponentBeginOverlap(Box)
  (params (OverlappedComponent :type Primitive%20Component%20Object%20Reference) (OtherActor :type Actor%20Object%20Reference) (OtherComp :type Primitive%20Component%20Object%20Reference) (OtherBodyIndex :type Integer) (bFromSweep :type Boolean) (SweepResult :type Hit%20Result%20Structure%20%28by%20ref%29))
  (Timeline|update Play
    (:Update
      (bind _outhit (Collision|BoxTraceByChannel (Transformation|GetWorldLocation (Variables|Default|GetStart)) (Transformation|GetWorldLocation (Variables|Default|GetEnd)) "30.000000,75.000000,35.000000" "0, 0, 0" "TraceTypeQuery1" false 0 "None"))
      (bind _output_get (Variables|Default|SetDistance (Math|Float|NormalizetoRange (.Distance (Collision|BreakHitResult _outhit)) 0.0 (Variables|Default|GetMaxDist))))
      (Default|SetPlayerScale (Variables|Default|GetPlayerRef) (Math|Vector|MakeVector (Math|Float|Lerp 1.0 (Variables|Default|GetTaille%20min) _output_get) (Math|Float|Lerp 1.0 (Variables|Default|GetTaille%20min) _output_get) (Math|Float|Lerp 1.0 (Variables|Default|GetTaille%20min) _output_get))))))

(event OnComponentEndOverlap(Box)
  (params (OverlappedComponent :type Primitive%20Component%20Object%20Reference) (OtherActor :type Actor%20Object%20Reference) (OtherComp :type Primitive%20Component%20Object%20Reference) (OtherBodyIndex :type Integer))
  (Timeline|update Stop
    (:Update
      (bind _outhit (Collision|BoxTraceByChannel (Transformation|GetWorldLocation (Variables|Default|GetStart)) (Transformation|GetWorldLocation (Variables|Default|GetEnd)) "30.000000,75.000000,35.000000" "0, 0, 0" "TraceTypeQuery1" false 0 "None"))
      (bind _output_get (Variables|Default|SetDistance (Math|Float|NormalizetoRange (.Distance (Collision|BreakHitResult _outhit)) 0.0 (Variables|Default|GetMaxDist))))
      (Default|SetPlayerScale (Variables|Default|GetPlayerRef) (Math|Vector|MakeVector (Math|Float|Lerp 1.0 (Variables|Default|GetTaille%20min) _output_get) (Math|Float|Lerp 1.0 (Variables|Default|GetTaille%20min) _output_get) (Math|Float|Lerp 1.0 (Variables|Default|GetTaille%20min) _output_get))))))

(event EventBeginPlay
  (bind _outhit (Collision|LineTraceByChannel (Transformation|GetWorldLocation (Variables|Default|GetStart)) (Transformation|GetWorldLocation (Variables|Default|GetEnd)) "TraceTypeQuery1" false (Variables|Default|GetActors%20to%20Ignore) "None" false))
  (Variables|Default|SetMaxDist (.Distance (Collision|BreakHitResult _outhit)))
  (bind _asbp_first_person_character (Utilities|Casting|CastToBP_FirstPersonCharacter (Game|Player|GetPlayerPawn 0)))
  (Variables|Default|SetPlayerRef _asbp_first_person_character))

(fn ConstructionScript)