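; Non-Euclidean portal actor that shows a linked camera's view and teleports the player through it.
; While the player is inside the render trigger, Tick mirrors the player camera's portal-relative transform onto the target, and the portal displays that render-target material.
; Overlapping the teleport trigger moves the player to that mirrored transform and matches yaw.
; Construction links a spline to the target; non-rendered portals drop the mesh and use an invisible teleport target.
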(event OnComponentBeginOverlap(TPtrigger)
  (params (OverlappedComponent :type Primitive%20Component%20Object%20Reference) (OtherActor :type Actor%20Object%20Reference) (OtherComp :type Primitive%20Component%20Object%20Reference) (OtherBodyIndex :type Integer) (bFromSweep :type Boolean) (SweepResult :type Hit%20Result%20Structure%20%28by%20ref%29))
  (if (not (Variables|Default|Getb_IsInvisible))
    (bind _asbp_first_person_character (Utilities|Casting|CastToBP_FirstPersonCharacter OtherActor))
    (if (not (== (Variables|/Game/Blueprints/BP_FirstPersonCharacter.BP_FirstPersonCharacter_C|GetCapsuleMonster _asbp_first_person_character) OtherComp))
      (CallFunction|TPActor OtherActor))))

(event OnComponentBeginOverlap(TriggerForRender)
  (params (OverlappedComponent :type Primitive%20Component%20Object%20Reference) (OtherActor :type Actor%20Object%20Reference) (OtherComp :type Primitive%20Component%20Object%20Reference) (OtherBodyIndex :type Integer) (bFromSweep :type Boolean) (SweepResult :type Hit%20Result%20Structure%20%28by%20ref%29))
  ;[1 1 1] Suivant si le joueur est ou n'est pas dans la zone change le matérial du portail
  (Utilities|Casting|CastToBP_FirstPersonCharacter OtherActor)
  (Variables|Default|Setb_MustRender true)
  (if (not (Variables|Default|Getb_DontRenderedPortal))
    (Rendering|Material|SetMaterial (Variables|Default|GetPortal) 0 (Variables|Default|GetMaterialOfTargetCam))))

(event OnComponentEndOverlap(TriggerForRender)
  (params (OverlappedComponent :type Primitive%20Component%20Object%20Reference) (OtherActor :type Actor%20Object%20Reference) (OtherComp :type Primitive%20Component%20Object%20Reference) (OtherBodyIndex :type Integer))
  ;[1 1 1] Suivant si le joueur est ou n'est pas dans la zone change le matérial du portail
  (Utilities|Casting|CastToBP_FirstPersonCharacter OtherActor)
  (Variables|Default|Setb_MustRender false)
  (if (not (Variables|Default|Getb_DontRenderedPortal))
    (Rendering|Material|SetMaterial (Variables|Default|GetPortal) 0 "/Game/ModularProps/Material_002.Material_002")))

(event EventTick
  (params (DeltaSeconds :type Float%20%28single-precision%29))
  (if (Variables|Default|Getb_MustRender)
    (CallFunction|RenderCambyPlayer)))

(fn ConstructionScript
  (if (not (Variables|Default|Getb_DontRenderedPortal))
    ;[1 1 1] Si il y a une caméra target alors rajoute un trait entre eux et change son matérial suivant la texture de la cam
    (bind _targetcamref (Variables|Default|GetTargetCamRef)
      (:then
        (bind _returnvalue (AddComponent|AddSplineComponent false))
        (Spline|SetLocationatSplinePoint _returnvalue 1 (Transformation|GetWorldLocation (Variables|/Game/Blueprints/Non-Euclidian/BP_CamRenderer.BP_CamRenderer_C|GetDefaultSceneRoot _targetcamref)) "World" true)
        (CallFunction|SetPortalMaterial))
      (:else))
    (else
      ;[1 1 1] Détruit le rendu du matérial si on n'en as pas besoin
      (bind _portal (Variables|Default|GetPortal)
        (:then
          (Components|DestroyComponent _portal)
          (bind _targetinvisibletpref (Variables|Default|GetTargetInvisibleTPRef)
            (:then
              (bind _returnvalue_2 (AddComponent|AddSplineComponent false))
              (Spline|SetLocationatSplinePoint _returnvalue_2 1 (Transformation|GetWorldLocation (Variables|/Script/Engine.Actor|GetRootComponent _targetinvisibletpref)) "World" true))
            (:else)))
        (:else))))
  ;[1 1 1] Change entre visible et invisible suivant les besoins
  (if (not (Variables|Default|Getb_IsInvisible))
    (Rendering|SetVisibility (Variables|Default|GetDefaultSceneRoot) true true)
    (else
      (Rendering|SetVisibility (Variables|Default|GetDefaultSceneRoot) false true))))

(fn SetPortalMaterial
  (bind _array_element (Utilities|Array|ForEachLoopwithBreak (Variables|Default|GetMaterialCamTargetArray) :!label _label)
    (:LoopBody
      (if (Utilities|Enum|Equal(Enum) (Utilities|GetObjectName _array_element) (Variables|/Game/Blueprints/Non-Euclidian/BP_CamRenderer.BP_CamRenderer_C|GetNameofTextureTargetRender (Variables|Default|GetTargetCamRef)))
        (Variables|Default|SetMaterialOfTargetCam _array_element)
        (Rendering|Material|SetMaterial (Variables|Default|GetPortal) 0 _array_element)
        (goto _label Break)))))

(fn RenderCambyPlayer
  (bind _returnvalue (Game|GetPlayerCameraManager 0))
  (bind _returnvalue_2 (Game|GetPlayerCameraManager 0))
  (bind _camtarget (Variables|Default|GetCamTarget))
  (bind _camtarget_2 (Variables|Default|GetCamTarget))
  (bind _transformcomponent (Variables|/Script/Engine.PlayerCameraManager|GetTransformComponent _returnvalue))
  (bind _transformcomponent_2 (Variables|/Script/Engine.PlayerCameraManager|GetTransformComponent _returnvalue_2))
  (if (not (Variables|Default|Getb_DontRenderedPortal))
    ;[1 1 1] Met la target de la camera au niveau de la caméra du player
    (Transformation|SetWorldLocationAndRotation (Variables|Default|GetCamTarget) (Transformation|GetWorldLocation _transformcomponent) (Transformation|GetWorldRotation _transformcomponent) false false)
    ;[1 1 1] Change la position de la caméra qui nous donne la texture au niveau de la position relative de la cam target
    (Transformation|SetRelativeLocationAndRotation (Variables|/Game/Blueprints/Non-Euclidian/BP_CamRenderer.BP_CamRenderer_C|GetCamRenderer (Variables|Default|GetTargetCamRef)) (Variables|/Script/Engine.SceneComponent|GetRelativeLocation _camtarget) (Variables|/Script/Engine.SceneComponent|GetRelativeRotation _camtarget) false false)
    (else
      (Transformation|SetWorldLocationAndRotation (Variables|Default|GetCamTarget) (Transformation|GetWorldLocation _transformcomponent_2) (Transformation|GetWorldRotation _transformcomponent_2) false false)
      (Transformation|SetRelativeLocationAndRotation (Variables|/Game/Blueprints/Non-Euclidian/BP_TPInvisible.BP_TPInvisible_C|GetTPTarget_0 (Variables|Default|GetTargetInvisibleTPRef)) (Variables|/Script/Engine.SceneComponent|GetRelativeLocation _camtarget_2) (Variables|/Script/Engine.SceneComponent|GetRelativeRotation _camtarget_2) false false))))

(fn TPActor
  (params (TargetTP :type Actor%20Object%20Reference))
  (bind _targetcamref (Variables|Default|GetTargetCamRef))
  (bind _targetinvisibletpref (Variables|Default|GetTargetInvisibleTPRef))
  (bind _camrenderer (Variables|/Game/Blueprints/Non-Euclidian/BP_CamRenderer.BP_CamRenderer_C|GetCamRenderer _targetcamref))
  (bind _tptarget_0 (Variables|/Game/Blueprints/Non-Euclidian/BP_TPInvisible.BP_TPInvisible_C|GetTPTarget_0 _targetinvisibletpref))
  (bind _returnvalue (Transformation|GetWorldLocation _tptarget_0))
  (bind _returnvalue_2 (Transformation|GetWorldLocation _camrenderer))
  (if (not (Variables|Default|Getb_DontRenderedPortal))
    ;[1 1 1] Téléporte l'acteur au niveau de Camrenderer
    (Transformation|Teleport TargetTP (Math|Vector|MakeVector (+ (Variables|Default|GetOffsetTP) (.x _returnvalue_2)) (.y _returnvalue_2) (+ (.z _returnvalue_2) -151.327179)) "0, 0, 0")
    (Pawn|SetControlRotation (Game|GetPlayerController 0) (Math|Rotator|MakeRotator 0.0 0.0 (.yaw (Transformation|GetWorldRotation _camrenderer))))
    (return)
    (else
      ;[1 1 1] Téléporte l'acteur au niveau de Camrenderer
      (Transformation|Teleport TargetTP (Math|Vector|MakeVector (+ (Variables|Default|GetOffsetTP) (.x _returnvalue)) (.y _returnvalue) (+ (.z _returnvalue) -151.327179)) "0, 0, 0")
      (Pawn|SetControlRotation (Game|GetPlayerController 0) (Math|Rotator|MakeRotator 0.0 0.0 (.yaw (Transformation|GetWorldRotation _tptarget_0))))
      (return))))