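; BP_Render drives a render-to-texture camera, CameraRender, in the Non-Euclidian Blueprint set.
; On BeginPlay, SetRenderSize resizes the camera's target texture to the current viewport width and height.
; StartRender and StopRender events switch capture updates on and off by toggling the component's tick, printing a debug message each time.
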(event Custom|SetRenderSize
  (bind _returnvalue (Viewport|GetViewportSize))
  (Settings|GetGameUserSettings)
  (Rendering|ResizeRenderTarget2D (Variables|/Script/Engine.SceneCaptureComponent2D|GetTextureTarget (Variables|Default|GetCameraRender)) (Math|Float|Truncate (.x _returnvalue)) (Math|Float|Truncate (.y _returnvalue))))

(event Custom|StopRender
  (Components|Tick|SetComponentTickEnabled (Variables|Default|GetCameraRender) false)
  (Development|PrintString "Stop render"))

(event Custom|StartRender
  (Components|Tick|SetComponentTickEnabled (Variables|Default|GetCameraRender) true)
  (Development|PrintString "Start render"))

(event EventBeginPlay
  (CallFunction|SetRenderSize))

(fn ConstructionScript)