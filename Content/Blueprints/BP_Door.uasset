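; BP_Door is an interactable door with default, locked, key, one-sided and open-once types, animated by timelines rotating two door meshes.
; Interact can first swap a disappearing actor for an appearing one, then CheckType opens, closes or refuses the door, using a trigger for side detection.
; A set ConnectedTo adds connected open/close events.
; Optional auto-close re-checks its trigger after a delay until clear, while UnlockDoor resets the type and removes the key.
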(event OnComponentBeginOverlap(TriggerGoodSide)
  (params (OverlappedComponent :type Primitive%20Component%20Object%20Reference) (OtherActor :type Actor%20Object%20Reference) (OtherComp :type Primitive%20Component%20Object%20Reference) (OtherBodyIndex :type Integer) (bFromSweep :type Boolean) (SweepResult :type Hit%20Result%20Structure%20%28by%20ref%29))
  (Utilities|Casting|CastToBP_FirstPersonCharacter OtherActor)
  (Variables|Default|Setb_GoodSide true))

(event OnComponentEndOverlap(TriggerGoodSide)
  (params (OverlappedComponent :type Primitive%20Component%20Object%20Reference) (OtherActor :type Actor%20Object%20Reference) (OtherComp :type Primitive%20Component%20Object%20Reference) (OtherBodyIndex :type Integer))
  (Utilities|Casting|CastToBP_FirstPersonCharacter OtherActor)
  (Variables|Default|Setb_GoodSide false))

(event OnComponentBeginOverlap(TriggerCloseDoor)
  (params (OverlappedComponent :type Primitive%20Component%20Object%20Reference) (OtherActor :type Actor%20Object%20Reference) (OtherComp :type Primitive%20Component%20Object%20Reference) (OtherBodyIndex :type Integer) (bFromSweep :type Boolean) (SweepResult :type Hit%20Result%20Structure%20%28by%20ref%29))
  (if (Variables|Default|Getb_CloseAfterEntry)
    (bind _asbp_first_person_character (Utilities|Casting|CastToBP_FirstPersonCharacter OtherActor))
    (if (not (== (Variables|/Game/Blueprints/BP_FirstPersonCharacter.BP_FirstPersonCharacter_C|GetMonster _asbp_first_person_character) OtherComp))
      (Utilities|FlowControl|Delay (Variables|Default|GetDelayBeforeCloseDoor))
      (if (Collision|IsOverlappingActor (Variables|Default|GetTriggerCloseDoor) OtherActor :!class /Script/Engine.PrimitiveComponent)
        (CallFunction|CheckIsonDoor)
        (else
          (Variables|Default|GetConnectedTo
            (:then
              (Utilities|FlowControl|Sequence
                (:then_0
                  (CallFunction|CloseConnectedDoor))
                (:then_1
                  _)))
            (:else
              _))
          (CallFunction|CloseDoor))))))

(event Custom|Interact
  (if (Variables|Default|GetNeedToDiseapearWall)
    (bind _disepear (Variables|Default|GetDisepear)
      (:then
        (Actor|DestroyActor _disepear)
        (Variables|Default|SetNeedToDiseapearWall false)
        (bind _appear (Variables|Default|GetAppear)
          (:then
            (Rendering|SetVisibility (Variables|/Script/Engine.StaticMeshActor|GetStaticMeshComponent _appear) true false)
            (Collision|SetCollisionEnabled (Variables|/Script/Engine.StaticMeshActor|GetStaticMeshComponent _appear) "QueryAndProbe"))
          (:else
            _))
        (CallFunction|CheckType))
      (:else
        (CallFunction|CheckType :!label _label)))
    (else
      (goto _label))))

(event Custom|CloseDoorAnim)

(event Custom|UnlockDoor
  (Variables|Default|SetDoorType "NewEnumerator0")
  (bind _key (Variables|Default|GetKey)
    (:then
      (Components|DestroyComponent _key))
    (:else)))

(event Custom|OpenConnectedDoor
  (if (not (Variables|Default|Getb_IsOpen))
    (Variables|Default|Setb_IsOpen true)
    (Utilities|FlowControl|Sequence
      (:then_0
        (bind _newtrack_0 (Timeline|Timeline_1 Play)
          (:Update
            (Transformation|SetRelativeRotation (Variables|Default|Getdoor1_door) (Math|Rotator|MakeRotator 0.0 0.0 (Math|Float|Lerp 0.0 9e+01 _newtrack_0)) false false))))
      (:then_1
        (bind _newtrack_0_2 (Timeline|Timeline_2 Play)
          (:Update
            (Transformation|SetRelativeRotation (Variables|Default|Getporte_gauche) (Math|Rotator|MakeRotator 0.0 0.0 (Math|Float|Lerp 0.0 -9e+01 _newtrack_0_2)) false false)))))
    (else
      (Variables|Default|Setb_IsOpen false)
      (Utilities|FlowControl|Sequence
        (:then_0
          (Timeline|Timeline_1 Reverse))
        (:then_1
          (Timeline|Timeline_2 Reverse))))))

(event Custom|OpenScriptedDoor
  (CallFunction|OpenCloseDoor))

(event Custom|OpenCloseDoor
  (bind _littles_walls_wall_6x6_006 (Variables|Default|GetLittles_Walls_Wall_6x6_006))
  (Variables|Default|GetConnectedTo
    (:then
      (Utilities|FlowControl|Sequence
        (:then_0
          (CallFunction|OpenConnectedDoor))
        (:then_1
          _)))
    (:else
      _))
  (if (not (Variables|Default|Getb_IsOpen))
    (Variables|Default|Setb_IsOpen true)
    (Utilities|FlowControl|Sequence
      (:then_0
        (bind _newtrack_0 (Timeline|Timeline Play)
          (:Update
            (Transformation|SetRelativeRotation (Variables|Default|Getdoor1_door) (Math|Rotator|MakeRotator 0.0 0.0 (Math|Float|Lerp 0.0 9e+01 _newtrack_0)) false false)
            (if (Variables|Default|Getb_IsOpen)
              (Physics|SetSimulatePhysics _littles_walls_wall_6x6_006 true)
              (Collision|SetCollisionEnabled _littles_walls_wall_6x6_006 "QueryAndPhysics")))))
      (:then_1
        (bind _newtrack_0_2 (Timeline|Timeline_0 Play)
          (:Update
            (Transformation|SetRelativeRotation (Variables|Default|Getporte_gauche) (Math|Rotator|MakeRotator 0.0 0.0 (Math|Float|Lerp 9e+01 0.0 _newtrack_0_2)) false false)))))
    (else
      (Variables|Default|Setb_IsOpen false)
      (Utilities|FlowControl|Sequence
        (:then_0
          (Timeline|Timeline Reverse))
        (:then_1
          (Timeline|Timeline_0 Reverse))))))

(event Custom|CloseDoor
  (bind _littles_walls_wall_6x6_006 (Variables|Default|GetLittles_Walls_Wall_6x6_006))
  (Variables|Default|Setb_IsOpen false)
  (Utilities|FlowControl|Sequence
    (:then_0
      (bind _newtrack_0 (Timeline|Timeline Reverse)
        (:Update
          (Transformation|SetRelativeRotation (Variables|Default|Getdoor1_door) (Math|Rotator|MakeRotator 0.0 0.0 (Math|Float|Lerp 0.0 9e+01 _newtrack_0)) false false)
          (if (Variables|Default|Getb_IsOpen)
            (Physics|SetSimulatePhysics _littles_walls_wall_6x6_006 true)
            (Collision|SetCollisionEnabled _littles_walls_wall_6x6_006 "QueryAndPhysics")))))
    (:then_1
      (bind _newtrack_0_2 (Timeline|Timeline_0 Reverse)
        (:Update
          (Transformation|SetRelativeRotation (Variables|Default|Getporte_gauche) (Math|Rotator|MakeRotator 0.0 0.0 (Math|Float|Lerp 9e+01 0.0 _newtrack_0_2)) false false))))))

(event Custom|CheckIsOnDoor
  (Utilities|FlowControl|Delay (Variables|Default|GetDelayBeforeCloseDoor))
  (if (Collision|IsOverlappingActor (Variables|Default|GetTriggerCloseDoor) (stale OnComponentBeginOverlap(TriggerCloseDoor) OtherActor) :!class /Script/Engine.PrimitiveComponent)
    (CallFunction|CheckIsonDoor)
    (else
      (Variables|Default|GetConnectedTo
        (:then
          (Utilities|FlowControl|Sequence
            (:then_0
              (CallFunction|CloseConnectedDoor))
            (:then_1
              _)))
        (:else
          _))
      (CallFunction|CloseDoor))))

(event Custom|Check%20Type
  (switch Utilities|FlowControl|Switch|SwitchonEnum_TypeOfDoor (Variables|Default|GetDoorType)
    (:NewEnumerator0
      (CallFunction|OpenCloseDoor))
    (:NewEnumerator1
      (CallFunction|CloseDoorAnim :!label _label))
    (:NewEnumerator2
      (goto _label))
    (:NewEnumerator3
      (if (Variables|Default|Getb_GoodSide)
        (CallFunction|OpenCloseDoor)
        (else
          (CallFunction|CloseDoorAnim))))
    (:NewEnumerator4
      (CallFunction|OpenCloseDoor)
      (Variables|Default|SetDoorType "NewEnumerator1"))))

(event Custom|CloseConnectedDoor
  (Variables|Default|Setb_IsOpen false)
  (Utilities|FlowControl|Sequence
    (:then_0
      (bind _newtrack_0 (Timeline|Timeline_1 Reverse)
        (:Update
          (Transformation|SetRelativeRotation (Variables|Default|Getdoor1_door) (Math|Rotator|MakeRotator 0.0 0.0 (Math|Float|Lerp 0.0 9e+01 _newtrack_0)) false false))))
    (:then_1
      (bind _newtrack_0_2 (Timeline|Timeline_2 Reverse)
        (:Update
          (Transformation|SetRelativeRotation (Variables|Default|Getporte_gauche) (Math|Rotator|MakeRotator 0.0 0.0 (Math|Float|Lerp 0.0 -9e+01 _newtrack_0_2)) false false))))))

(fn ConstructionScript
  (switch Utilities|FlowControl|Switch|SwitchonEnum_TypeOfDoor (Variables|Default|GetDoorType)
    (:NewEnumerator0
      (Components|DestroyComponent (Variables|Default|GetKey) :!label _label))
    (:NewEnumerator1
      (goto _label))
    (:NewEnumerator2
      (Rendering|SetVisibility (Variables|Default|GetLittles_Walls_Wall_6x6_006) true false))
    (:NewEnumerator3
      (goto _label))
    (:NewEnumerator4
      (goto _label))))

(fn ResetAllConected
  (bind _outactors (Actor|GetAllActorsOfClass "BP_Door_C"))
  (for _array_element _outactors
    (Variables|BP_Door_C|SetConnectedTo _array_element 0)))