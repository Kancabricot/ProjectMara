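; BP_Encen is a Blueprint that removes a stored set of actors from the game when its OnActive event fires.
; The event loops through ArrayToDestroy, destroys each valid actor and then clears the array, so later activations do nothing unless it is refilled.
; A debug print is left unconnected, and the construction script is empty.
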(event Custom|OnActive
  (if (not (Utilities|Array|IsEmpty (Variables|Default|GetArrayToDestroy)))
    (for _array_element (Variables|Default|GetArrayToDestroy)
      (Variables|Default|SetCurrentDestroy _array_element)
      (bind _currentdestroy (Variables|Default|GetCurrentDestroy)
        (:then
          (Actor|DestroyActor _currentdestroy))
        (:else)))
    (Utilities|Array|Clear (Variables|Default|GetArrayToDestroy))))

(fn ConstructionScript)