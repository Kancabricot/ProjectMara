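; BP_ObjectMemory is an object "memory" that hands its shape selection to the caller, apparently for morphing.
; The construction script maps SelectionObjectMemory to one of four static meshes, stores it in MemoryObjetToMorph and applies it to the ObjectMemory component.
; GetObjectEvent destroys the referenced ObjectToDestroy actor and the ObjectMemory component, then returns the selection.
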(fn ConstructionScript
  (switch Utilities|FlowControl|Switch|SwitchonEnum_ObjectMemory (Variables|Default|GetSelectionObject%20memory)
    (:NewEnumerator0
      (Variables|Default|SetMemoryObjetToMorph "/Engine/Functions/Engine_MaterialFunctions02/SupportFiles/1x1x1_Box_Pivot_-XYZ.1x1x1_Box_Pivot_-XYZ"))
    (:NewEnumerator1
      (Variables|Default|SetMemoryObjetToMorph "/Game/Assets/Props/Decoration/Bougie_2_bol.Bougie_2_bol"))
    (:NewEnumerator2
      (Variables|Default|SetMemoryObjetToMorph "/Game/Assets/Props/meubles/autel.autel"))
    (:NewEnumerator3
      (Variables|Default|SetMemoryObjetToMorph "/Engine/VREditor/TransformGizmo/BoundingBoxEdge.BoundingBoxEdge")))
  (Components|StaticMesh|SetStaticMesh (Variables|Default|GetObjectMemory) (Variables|Default|GetMemoryObjetToMorph)))

(fn GetObjectEvent
  (Actor|DestroyActor (Variables|Default|GetObjectToDestroy))
  (Components|DestroyComponent (Variables|Default|GetObjectMemory))
  (return (Variables|Default|GetSelectionObject%20memory)))