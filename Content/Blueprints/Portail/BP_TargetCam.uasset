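; Portal camera actor that captures the scene into a render target through its CamRenderer component.
; The construction script assigns TextureTargetRender to the capture and stores that asset's name with a "_Mat" suffix, apparently a matching material name.
; On BeginPlay it resizes the render target to the viewport's dimensions so the captured image matches screen resolution.
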(event EventBeginPlay
  (bind _returnvalue (Viewport|GetViewportSize))
  (Settings|GetGameUserSettings)
  (Rendering|ResizeRenderTarget2D (Variables|/Script/Engine.SceneCaptureComponent2D|GetTextureTarget (Variables|Default|GetCamRenderer)) (Math|Float|Truncate (.x _returnvalue)) (Math|Float|Truncate (.y _returnvalue))))

(fn ConstructionScript
  (Variables|/Script/Engine.SceneCaptureComponent2D|SetTextureTarget (Variables|Default|GetCamRenderer) (Variables|Default|GetTexture%20Target%20Render))
  (Variables|Default|SetNameofTextureTargetRender (Utilities|String|Append (Utilities|GetObjectName (Variables|Default|GetTexture%20Target%20Render)) "_Mat")))