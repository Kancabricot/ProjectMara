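; BP_CamRenderer is a capture camera actor that renders into a render target for the portal system.
; Its construction script assigns TextureTargetRender to the CamRenderer component and builds the linked material's name by appending "_Mat" to the texture's name.
; It then calls SetPortalMaterial on every PB_Portal in the level so each refreshes its material.
; At BeginPlay, it resizes the render target to the viewport size.
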(event EventBeginPlay
  (bind _returnvalue (Viewport|GetViewportSize))
  ;[1 1 1] Change le taille de la texture suivant la taille de l'écran
  (Settings|GetGameUserSettings)
  (Rendering|ResizeRenderTarget2D (Variables|/Script/Engine.SceneCaptureComponent2D|GetTextureTarget (Variables|Default|GetCamRenderer)) (Math|Float|Truncate (.x _returnvalue)) (Math|Float|Truncate (.y _returnvalue))))

(fn ConstructionScript
  ;[1 1 1] Chande la texture
  (Variables|/Script/Engine.SceneCaptureComponent2D|SetTextureTarget (Variables|Default|GetCamRenderer) (Variables|Default|GetTexture%20Target%20Render))
  ;[1 1 1] Récupere le nom de la texture pour trouver le material qui lui est lié
  (Variables|Default|SetNameofTextureTargetRender (Utilities|String|Append (Utilities|GetObjectName (Variables|Default|GetTexture%20Target%20Render)) "_Mat"))
  ;[1 1 1] Met à jour les portailles
  (bind _outactors (Actor|GetAllActorsOfClass "/Game/Blueprints/Portail/PB_Portal.PB_Portal_C"))
  (for _array_element _outactors
    (Default|SetPortalMaterial _array_element)))