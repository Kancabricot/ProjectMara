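; PB_Portal is a portal actor that shows a live view from a linked TargetCamRef and teleports overlapping actors to that camera, with an offset.
; While the first-person character is inside the render trigger, Tick copies the player camera's transform, relative to this portal, onto the target's capture camera.
; The trigger also swaps the portal to the target's material, matched by name in the construction script, which draws a spline to the target.
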(event OnComponentBeginOverlap(TPtrigger)
  (params (OverlappedComponent :type Primitive%20Component%20Object%20Reference) (OtherActor :type Actor%20Object%20Reference) (OtherComp :type Primitive%20Component%20Object%20Reference) (OtherBodyIndex :type Integer) (bFromSweep :type Boolean) (SweepResult :type Hit%20Result%20Structure%20%28by%20ref%29))
  (bind _targetcamref (Variables|Default|GetTargetCamRef))
  (bind _camrenderer (Variables|/Game/Blueprints/Portail/BP_TargetCam.BP_TargetCam_C|GetCamRenderer _targetcamref))
  (bind _returnvalue (Transformation|GetWorldLocation _camrenderer))
  (Transformation|Teleport OtherActor (Math|Vector|MakeVector (+ (Variables|Default|GetOffsetTP) (.x _returnvalue)) (.y _returnvalue) (+ (.z _returnvalue) -151.327179)) (Transformation|GetWorldRotation _camrenderer)))

(event OnComponentBeginOverlap(TriggerForRender)
  (params (OverlappedComponent :type Primitive%20Component%20Object%20Reference) (OtherActor :type Actor%20Object%20Reference) (OtherComp :type Primitive%20Component%20Object%20Reference) (OtherBodyIndex :type Integer) (bFromSweep :type Boolean) (SweepResult :type Hit%20Result%20Structure%20%28by%20ref%29))
  (Utilities|Casting|CastToBP_FirstPersonCharacter OtherActor)
  (Variables|Default|Setb_MustRender true)
  (if (not (Variables|Default|Getb_DontRenderedPortal))
    (Rendering|Material|SetMaterial (Variables|Default|GetPortal) 0 (Variables|Default|GetMaterialOfTargetCam))))

(event OnComponentEndOverlap(TriggerForRender)
  (params (OverlappedComponent :type Primitive%20Component%20Object%20Reference) (OtherActor :type Actor%20Object%20Reference) (OtherComp :type Primitive%20Component%20Object%20Reference) (OtherBodyIndex :type Integer))
  (Utilities|Casting|CastToBP_FirstPersonCharacter OtherActor)
  (Variables|Default|Setb_MustRender false)
  (if (not (Variables|Default|Getb_DontRenderedPortal))
    (Rendering|Material|SetMaterial (Variables|Default|GetPortal) 0 "/Game/ModularProps/Material_002.Material_002")))

(event EventBeginPlay
  (if (not (Variables|Default|Getb_DontRenderedPortal))
    (Rendering|Material|SetMaterial (Variables|Default|GetPortal) 0 "/Game/ModularProps/Material_002.Material_002")))

(event EventTick
  (params (DeltaSeconds :type Float%20%28single-precision%29))
  (bind _returnvalue (Game|GetPlayerCameraManager 0))
  (bind _camtarget (Variables|Default|GetCamTarget))
  (bind _transformcomponent (Variables|/Script/Engine.PlayerCameraManager|GetTransformComponent _returnvalue))
  (if (Variables|Default|Getb_MustRender)
    (Transformation|SetWorldLocationAndRotation (Variables|Default|GetCamTarget) (Transformation|GetWorldLocation _transformcomponent) (Transformation|GetWorldRotation _transformcomponent) false false)
    (Transformation|SetRelativeLocationAndRotation (Variables|/Game/Blueprints/Portail/BP_TargetCam.BP_TargetCam_C|GetCamRenderer (Variables|Default|GetTargetCamRef)) (Variables|/Script/Engine.SceneComponent|GetRelativeLocation _camtarget) (Variables|/Script/Engine.SceneComponent|GetRelativeRotation _camtarget) false false)))

(fn ConstructionScript
  (bind _targetcamref (Variables|Default|GetTargetCamRef))
  (bind _nameoftexturetargetrender (Variables|/Game/Blueprints/Portail/BP_TargetCam.BP_TargetCam_C|GetNameofTextureTargetRender _targetcamref))
  (if (not (Variables|Default|Getb_DontRenderedPortal))
    (bind _targetcamref_2 (Variables|Default|GetTargetCamRef)
      (:then
        (bind _returnvalue (AddComponent|AddSplineComponent false))
        (Spline|SetLocationatSplinePoint _returnvalue 1 (Transformation|GetWorldLocation (Variables|/Game/Blueprints/Portail/BP_TargetCam.BP_TargetCam_C|GetDefaultSceneRoot _targetcamref_2)) "World" true)
        (bind _array_element (Utilities|Array|ForEachLoopwithBreak (Variables|Default|GetMaterialCamTargetArray) :!label _label)
          (:LoopBody
            (if (Utilities|Enum|Equal(Enum) (Utilities|GetObjectName _array_element) _nameoftexturetargetrender)
              (Variables|Default|SetMaterialOfTargetCam _array_element)
              (Rendering|Material|SetMaterial (Variables|Default|GetPortal) 0 _array_element)
              (Development|PrintString "good name")
              (goto _label Break)
              (else
                (Development|PrintString (Utilities|GetObjectName _array_element))
                (Development|PrintString _nameoftexturetargetrender true true "(R=1.000000,G=0.000000,B=0.098743,A=1.000000)"))))))
      (:else))
    (else
      (Components|DestroyComponent (Variables|Default|GetPortal)))))