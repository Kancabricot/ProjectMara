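; BP_Autel is an altar that reveals placed memory objects and opens the scripted doors tied to them.
; Its PlaceObject event switches on a selection of four objects, unhiding the matching ObjectMemory component.
; It then calls OpenScriptedDoor on the corresponding door reference, provided that reference is valid.
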(event Custom|PlaceObject
  (params (Selection :type Enum_ObjectMemory%20Enum :default "NewEnumerator0"))
  (switch Utilities|FlowControl|Switch|SwitchonEnum_ObjectMemory Selection
    (:NewEnumerator0
      (Development|SetHiddeninGame (Variables|Default|GetObject%20Memory%201) false false)
      (bind _door1 (Variables|Default|GetDoor1)
        (:then
          (Default|OpenScriptedDoor _door1))
        (:else)))
    (:NewEnumerator1
      (Development|SetHiddeninGame (Variables|Default|GetObject%20Memory%202) false false)
      (bind _door2 (Variables|Default|GetDoor2)
        (:then
          (Default|OpenScriptedDoor _door2))
        (:else)))
    (:NewEnumerator2
      (Development|SetHiddeninGame (Variables|Default|GetObject%20Memory%203) false false)
      (bind _door3 (Variables|Default|GetDoor3)
        (:then
          (Default|OpenScriptedDoor _door3))
        (:else)))
    (:NewEnumerator3
      (Development|SetHiddeninGame (Variables|Default|GetObject%20Memory%204) false false)
      (bind _door4 (Variables|Default|GetDoor4)
        (:then
          (Default|OpenScriptedDoor _door4))
        (:else)))))

(fn ConstructionScript)