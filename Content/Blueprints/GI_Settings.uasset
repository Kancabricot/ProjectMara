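; GI_Settings, by its name a Game Instance, holds the player's display, audio and control settings plus quest progress, persisted in one BP_SaveGame slot.
; Load restores them from the save, or creates an empty save object if none exists.
; Resolution and screen-mode changes go through GameUserSettings, then resize BP_Render and save only if that actor exists.
; Volume uses a master sound-mix override, while PlaySound plays a fixed-location door bang and saves.
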(fn SetScreenResolution
  (bind _returnvalue (Settings|GetGameUserSettings))
  (Class|GameUserSettings|SetScreenResolution _returnvalue (Utilities|Array|Get(acopy) (Variables|Default|GetResolutionArray) (Variables|Default|GetIndexOfResolution)))
  (Class|GameUserSettings|ApplyResolutionSettings _returnvalue false)
  (Class|GameUserSettings|ApplySettings _returnvalue true)
  (bind _returnvalue_2 (Actor|GetActorOfClass "/Game/Blueprints/Non-Euclidian/BP_Render.BP_Render_C"))
  (Utilities|IsValid _returnvalue_2
    (:Is%20Valid
      (Default|SetRenderSize _returnvalue_2)
      (CallFunction|SaveSetting))))

(fn SetScreenMode
  (bind _returnvalue (Settings|GetGameUserSettings))
  (Class|GameUserSettings|SetFullscreenMode _returnvalue (Variables|Default|GetFullScreen))
  (Class|GameUserSettings|ApplySettings _returnvalue true)
  (bind _returnvalue_2 (Actor|GetActorOfClass "/Game/Blueprints/Non-Euclidian/BP_Render.BP_Render_C"))
  (Utilities|IsValid _returnvalue_2
    (:Is%20Valid
      (Default|SetRenderSize _returnvalue_2)
      (CallFunction|SaveSetting))))

(fn SetVolume
  (Audio|SetSoundMixClassOverride "/Game/Assets/SFX/SMC_Master.SMC_Master" "/Engine/EngineSounds/Master.Master" (Variables|Default|GetVolume) 1.0 1.0 true)
  (Audio|PushSoundMixModifier "/Game/Assets/SFX/SMC_Master.SMC_Master"))

(fn PlaySound
  (Audio|PlaySoundatLocation "/Game/Assets/SFX/Ambiance/WAVs/Door_bang_02.Door_bang_02" "256.189281,-474.975665,340.000000" "0, 0, 0" 1.0 1.0 0.0 0 0 0 0)
  (CallFunction|SaveSetting))

(fn SaveQuest
  (params (Quest :type Enum_ObjectMemory%20Enum :default "NewEnumerator0"))
  (bind _output_get (Variables|Default|SetQuest Quest))
  (Variables|/Game/Blueprints/Save/BP_SaveGame.BP_SaveGame_C|SetQuest (Variables|Default|GetSaveInstance) _output_get)
  (SaveGame|SaveGametoSlot (Variables|Default|GetSaveInstance) "Save"))

(fn SaveSetting
  (bind _saveinstance (Variables|Default|GetSaveInstance))
  (Variables|/Game/Blueprints/Save/BP_SaveGame.BP_SaveGame_C|SetCamShake _saveinstance (Variables|Default|GetCamShake))
  (Variables|/Game/Blueprints/Save/BP_SaveGame.BP_SaveGame_C|SetSensivity _saveinstance (Variables|Default|GetSensivity))
  (Variables|/Game/Blueprints/Save/BP_SaveGame.BP_SaveGame_C|SetFullScreen _saveinstance (Variables|Default|GetFullScreen))
  (Variables|/Game/Blueprints/Save/BP_SaveGame.BP_SaveGame_C|SetResolutionArray _saveinstance (Variables|Default|GetResolutionArray))
  (Variables|/Game/Blueprints/Save/BP_SaveGame.BP_SaveGame_C|SetIndexOfResolution _saveinstance (Variables|Default|GetIndexOfResolution))
  (Variables|/Game/Blueprints/Save/BP_SaveGame.BP_SaveGame_C|SetVolume _saveinstance (Variables|Default|GetVolume))
  (Variables|/Game/Blueprints/Save/BP_SaveGame.BP_SaveGame_C|SetLuminosity _saveinstance (Variables|Default|GetLuminosity))
  (Variables|/Game/Blueprints/Save/BP_SaveGame.BP_SaveGame_C|SetSelectedOption _saveinstance (Variables|Default|GetSelectedOption))
  (Variables|/Game/Blueprints/Save/BP_SaveGame.BP_SaveGame_C|SetInverseAxisY _saveinstance (Variables|Default|GetInverseAxisY))
  (Variables|/Game/Blueprints/Save/BP_SaveGame.BP_SaveGame_C|SetWASD _saveinstance (Variables|Default|GetWASD))
  (SaveGame|SaveGametoSlot (Variables|Default|GetSaveInstance) "Save"))

(fn CheckSave
  (bind _returnvalue (SaveGame|DoesSaveGameExist "Save"))
  (if _returnvalue
    ;[1 1 1] Récupere la sauvegarde
    (bind _returnvalue_2 (SaveGame|LoadGamefromSlot "Save"))
    (bind _asbp_save_game (Utilities|Casting|CastToBP_SaveGame _returnvalue_2))
    (Variables|Default|SetSaveInstance _asbp_save_game)
    (Development|PrintString "Have a save")
    (return true)
    (else
      (bind _returnvalue_3 (SaveGame|CreateSaveGameObject "/Game/Blueprints/Save/BP_SaveGame.BP_SaveGame_C"))
      (Variables|Default|SetSaveInstance _returnvalue_3)
      (return false))))

(fn Load
  (bind _saveinstance (Variables|Default|GetSaveInstance))
  (bind _b_havesave (CallFunction|CheckSave))
  (if _b_havesave
    (Variables|Default|SetCamShake (Variables|/Game/Blueprints/Save/BP_SaveGame.BP_SaveGame_C|GetCamShake _saveinstance))
    (Variables|Default|SetSensivity (Variables|/Game/Blueprints/Save/BP_SaveGame.BP_SaveGame_C|GetSensivity _saveinstance))
    (Variables|Default|SetFullScreen (Variables|/Game/Blueprints/Save/BP_SaveGame.BP_SaveGame_C|GetFullScreen _saveinstance))
    (Variables|Default|SetResolutionArray (Variables|/Game/Blueprints/Save/BP_SaveGame.BP_SaveGame_C|GetResolutionArray _saveinstance))
    (Variables|Default|SetIndexOfResolution (Variables|/Game/Blueprints/Save/BP_SaveGame.BP_SaveGame_C|GetIndexOfResolution _saveinstance))
    (Variables|Default|SetVolume (Variables|/Game/Blueprints/Save/BP_SaveGame.BP_SaveGame_C|GetVolume _saveinstance))
    (Variables|Default|SetLuminosity (Variables|/Game/Blueprints/Save/BP_SaveGame.BP_SaveGame_C|GetLuminosity _saveinstance))
    (Variables|Default|SetSelectedOption (Variables|/Game/Blueprints/Save/BP_SaveGame.BP_SaveGame_C|GetSelectedOption _saveinstance))
    (Variables|Default|SetInverseAxisY (Variables|/Game/Blueprints/Save/BP_SaveGame.BP_SaveGame_C|GetInverseAxisY _saveinstance))
    (Variables|Default|SetWASD (Variables|/Game/Blueprints/Save/BP_SaveGame.BP_SaveGame_C|GetWASD _saveinstance))
    (Variables|Default|SetQuest (Variables|/Game/Blueprints/Save/BP_SaveGame.BP_SaveGame_C|GetQuest _saveinstance))))