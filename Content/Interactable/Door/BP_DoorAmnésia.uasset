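; Amnesia-style interactive door that the player swings open and closed by turn input.
; OpenDoor yaws the door mesh by turn rate times sensitivity, inverting the direction when the player looks from the back side, and sets the player's TED flag.
; BeginPlay caches the first-person character and starting yaw, with no angle clamp applied here.
; Tick zeroes the turn rate when mouse X and the player are still.
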(event Custom|OpenDoor
  (params (TurnRate :type Float%20%28double-precision%29) (Sensi :type Float%20%28double-precision%29))
  (bind _door1_door (Variables|Default|Getdoor1_door))
  (bind _returnvalue (* (Variables|Default|GetTurnRate) Sensi))
  (bind _returnvalue_2 (Math|Rotator|MakeRotator 0.0 0.0 _returnvalue))
  (if (not (Variables|/Game/Blueprints/BP_FirstPersonCharacter.BP_FirstPersonCharacter_C|GetIsLookingFromBackSide (Variables|Default|GetPlayerRef)))
    (Transformation|AddLocalRotation _door1_door (Math|Rotator|MakeRotator 0.0 0.0 (.yaw _returnvalue_2)) false false)
    (else
      (Transformation|AddLocalRotation _door1_door (Math|Rotator|MakeRotator 0.0 0.0 (/ (.yaw _returnvalue_2) -1.0)) false false)))
  (Variables|/Game/Blueprints/BP_FirstPersonCharacter.BP_FirstPersonCharacter_C|SetTED (Variables|Default|GetPlayerRef) true))

(event EventTick
  (params (DeltaSeconds :type Float%20%28single-precision%29))
  (if (not (!= (.DeltaX (Class|PlayerController|GetInputMouseDelta (Game|GetPlayerController 0))) 0.0))
    (if (Variables|/Game/Blueprints/BP_FirstPersonCharacter.BP_FirstPersonCharacter_C|GetNotMooving (Variables|Default|GetPlayerRef))
      (Variables|Default|SetTurnRate 0.0))))

(event EventBeginPlay
  (Variables|Default|SetMinAngle (.yaw (Transformation|GetWorldRotation (Variables|Default|Getdoor1_door))))
  (bind _returnvalue (Actor|GetActorOfClass "/Game/Blueprints/BP_FirstPersonCharacter.BP_FirstPersonCharacter_C"))
  (Variables|Default|SetPlayerRef _returnvalue))

(fn ConstructionScript)