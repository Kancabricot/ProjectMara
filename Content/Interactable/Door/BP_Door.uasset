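; Interactable double door that swings both leaves on timelines, with optional key lock and one-side-only opening.
; An overlap box tracks the player's side; a blocked attempt just prints "Is locked", and unlocking removes the Key component.
; In open-once mode, a trigger locks and closes the door after a delay if the player is off that side.
; OpenConnectedDoor toggles without checks; ResetAllConected clears every door's link.
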(event OnComponentBeginOverlap(Box)
  (params (OverlappedComponent :type Primitive%20Component%20Object%20Reference) (OtherActor :type Actor%20Object%20Reference) (OtherComp :type Primitive%20Component%20Object%20Reference) (OtherBodyIndex :type Integer) (bFromSweep :type Boolean) (SweepResult :type Hit%20Result%20Structure%20%28by%20ref%29))
  (Utilities|Casting|CastToBP_FirstPersonCharacter OtherActor)
  (Variables|Default|Setb_GoodSide true))

(event OnComponentEndOverlap(Box)
  (params (OverlappedComponent :type Primitive%20Component%20Object%20Reference) (OtherActor :type Actor%20Object%20Reference) (OtherComp :type Primitive%20Component%20Object%20Reference) (OtherBodyIndex :type Integer))
  (Utilities|Casting|CastToBP_FirstPersonCharacter OtherActor)
  (Variables|Default|Setb_GoodSide false))

(event OnComponentBeginOverlap(TriggerCloseDoor)
  (params (OverlappedComponent :type Primitive%20Component%20Object%20Reference) (OtherActor :type Actor%20Object%20Reference) (OtherComp :type Primitive%20Component%20Object%20Reference) (OtherBodyIndex :type Integer) (bFromSweep :type Boolean) (SweepResult :type Hit%20Result%20Structure%20%28by%20ref%29))
  (if (Variables|Default|Getb_OpenOnce)
    (Utilities|Casting|CastToBP_FirstPersonCharacter OtherActor)
    (Utilities|FlowControl|Delay (Variables|Default|GetDelayBeforeCloseDoor))
    (if (not (Variables|Default|Getb_GoodSide))
      (Variables|Default|Setb_IsLock true)
      (Variables|Default|Setb_IsOpen false)
      (Utilities|FlowControl|Sequence
        (:then_0
          (bind _newtrack_0 (Timeline|Timeline Reverse)
            (:Update
              (Transformation|SetRelativeRotation (Variables|Default|Getdoor1_door) (Math|Rotator|MakeRotator 0.0 0.0 (Math|Float|Lerp 0.0 9e+01 _newtrack_0)) false false))))
        (:then_1
          (bind _newtrack_0_2 (Timeline|Timeline_0 Reverse)
            (:Update
              (Transformation|SetRelativeRotation (Variables|Default|Getporte_gauche) (Math|Rotator|MakeRotator 0.0 0.0 (Math|Float|Lerp 0.0 -9e+01 _newtrack_0_2)) false false))))))))

(event Custom|OpenDoor
  (if (not (Variables|Default|Getb_IsOpen))
    (if (not (Variables|Default|Getb_IsLock))
      (if (not (Variables|Default|Getb_OnlyOnSide))
        (Variables|Default|Setb_IsOpen true :!label _label)
        (Utilities|FlowControl|Sequence
          (:then_0
            (bind _newtrack_0 (Timeline|Timeline Play)
              (:Update
                (Transformation|SetRelativeRotation (Variables|Default|Getdoor1_door) (Math|Rotator|MakeRotator 0.0 0.0 (Math|Float|Lerp 0.0 9e+01 _newtrack_0)) false false))))
          (:then_1
            (bind _newtrack_0_2 (Timeline|Timeline_0 Play)
              (:Update
                (Transformation|SetRelativeRotation (Variables|Default|Getporte_gauche) (Math|Rotator|MakeRotator 0.0 0.0 (Math|Float|Lerp 0.0 -9e+01 _newtrack_0_2)) false false)))))
        (elif (Variables|Default|Getb_GoodSide)
          (goto _label)
          (else
            (CallFunction|CloseDoorEvent))))
      (else
        (CallFunction|CloseDoorEvent)))
    (else
      (Variables|Default|Setb_IsOpen false)
      (Utilities|FlowControl|Sequence
        (:then_0
          (Timeline|Timeline Reverse))
        (:then_1
          (Timeline|Timeline_0 Reverse))))))

(event Custom|CloseDoorEvent
  (Development|PrintString "Is locked"))

(event Custom|UnlockDoor
  (Variables|Default|Setb_IsLock false)
  (Components|DestroyComponent (Variables|Default|GetKey)))

(event Custom|OpenConnectedDoor
  ;[1 1 1] Open La porte avec avec laqulle elle est connecter
  (if (not (Variables|Default|Getb_IsOpen))
    (Utilities|FlowControl|Sequence
      (:then_0
        (Variables|Default|Setb_IsOpen true)
        (bind _newtrack_0 (Timeline|Timeline_1 Play)
          (:Update
            (Transformation|SetRelativeRotation (Variables|Default|Getdoor1_door) (Math|Rotator|MakeRotator 0.0 0.0 (Math|Float|Lerp 0.0 9e+01 _newtrack_0)) false false))))
      (:then_1
        (bind _newtrack_0_2 (Timeline|Timeline_2 Play)
          (:Update
            (Transformation|SetRelativeRotation (Variables|Default|Getporte_gauche) (Math|Rotator|MakeRotator 0.0 0.0 (Math|Float|Lerp 0.0 -9e+01 _newtrack_0_2)) false false)))))
    (else
      (Utilities|FlowControl|Sequence
        (:then_0
          (Variables|Default|Setb_IsOpen false)
          (Timeline|Timeline_1 Reverse))
        (:then_1
          (Timeline|Timeline_2 Reverse))))))

(fn ConstructionScript
  (if (not (Variables|Default|Getb_IsLock))
    (Components|DestroyComponent (Variables|Default|GetKey))))

(fn ResetAllConected
  (bind _outactors (Actor|GetAllActorsOfClass "BP_Door_C"))
  (for _array_element _outactors
    (Variables|BP_Door_C|SetConnectedTo _array_element 0)))